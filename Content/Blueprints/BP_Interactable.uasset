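; BP_Interactable is a mesh actor that cycles through a list of color and texture looks each time UpdateColor fires.
; The construction script creates a dynamic material on the Cube, applies the first Materials entry and sets the configurable mesh.
; UpdateColor loads the next wrapped entry as the New parameters, then a timeline drives LerpValue to blend toward it.
; On finish, New values become Current, and CanInteract, cleared during the blend, is restored.
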(event Custom|UpdateColor
  (bind _dynamat (Variables|Default|GetDynamat))
  (Variables|Default|SetCanInteract false)
  (CallFunction|SetNewColor)
  (bind _colorupdate (Timeline|Color PlayFromStart)
    (:Update
      (Rendering|Material|SetScalarParameterValue (Variables|Default|GetDynamat) "LerpValue" _colorupdate :!class /Script/Engine.MaterialInstanceDynamic))
    (:Finished
      (bind _returnvalue (Rendering|Material|GetVectorParameterValue _dynamat "NewColor" :!class /Script/Engine.MaterialInstanceDynamic))
      (Rendering|Material|SetVectorParameterValue _dynamat "CurrentColor" _returnvalue :!class /Script/Engine.MaterialInstanceDynamic)
      (bind _returnvalue_2 (Rendering|Material|GetTextureParameterValue _dynamat "NewTexture" :!class /Script/Engine.MaterialInstanceDynamic))
      (Rendering|Material|SetTextureParameterValue _dynamat "CurrentTexture" _returnvalue_2)
      (Variables|Default|SetCanInteract true))))

(fn ConstructionScript
  (bind _materials (Variables|Default|GetMaterials))
  (bind _output (Utilities|Array|Get(acopy) _materials))
  (bind (_color _texture) (Utilities|Struct|BreakStruct_ColorTexture _output))
  (bind _returnvalue (Rendering|Material|CreateDynamicMaterialInstance (Variables|Default|GetCube) 0 0 "None" :!class /Script/Engine.PrimitiveComponent))
  (Variables|Default|SetDynamat _returnvalue)
  (Rendering|Material|SetVectorParameterValue (Variables|Default|GetDynamat) "CurrentColor" _color :!class /Script/Engine.MaterialInstanceDynamic)
  (Rendering|Material|SetTextureParameterValue (Variables|Default|GetDynamat) "CurrentTexture" _texture)
  (Components|StaticMesh|SetStaticMesh (Variables|Default|GetCube) (Variables|Default|GetMesh)))

(fn SetNewColor
  (bind _dynamat (Variables|Default|GetDynamat))
  (if (< (Variables|Default|GetColorID) (- (Utilities|Array|Length (Variables|Default|GetMaterials)) 1))
    (Variables|Default|SetColorID (+ (Variables|Default|GetColorID) 1))
    (else
      (Variables|Default|SetColorID 0)))
  (Rendering|Material|SetVectorParameterValue _dynamat "NewColor" (.Color (Utilities|Struct|BreakStruct_ColorTexture (Utilities|Array|Get(acopy) (Variables|Default|GetMaterials) (Variables|Default|GetColorID)))) :!class /Script/Engine.MaterialInstanceDynamic)
  (Rendering|Material|SetTextureParameterValue _dynamat "NewTexture" (.Texture (Utilities|Struct|BreakStruct_ColorTexture (Utilities|Array|Get(acopy) (Variables|Default|GetMaterials) (Variables|Default|GetColorID))))))