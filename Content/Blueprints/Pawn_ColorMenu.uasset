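; Player pawn for a color-changing interaction setup, which adds the in-game UI to the viewport on BeginPlay.
; On Interact it traces 1000 units forward from the camera against world objects, drawing persistent debug lines.
; A hit BP_Interactable gets its color updated if it can be interacted with; otherwise a message reports that it is still changing colors.
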(event EventBeginPlay
  (bind _returnvalue (UserInterface|CreateWidget "/Game/UI/UI_Ingame.UI_Ingame_C" (Game|GetPlayerController 0)))
  (UserInterface|Viewport|AddtoViewport _returnvalue 0))

(event Input|ActionEvents|InputActionInteract
  (params (Key :type Key%20Structure))
  (bind _returnvalue (Game|GetPlayerCameraManager 0))
  (bind _returnvalue_2 (Transformation|GetActorLocation _returnvalue))
  (:Pressed
    (bind _outhit (Collision|LineTraceForObjects _returnvalue_2 (+ _returnvalue_2 (* (Transformation|GetActorForwardVector _returnvalue) 1e+03)) (Utilities|Array|MakeArray "ObjectTypeQuery1" "ObjectTypeQuery2") false 0 "Persistent"))
    (bind _asbp_interactable (Utilities|Casting|CastToBP_Interactable (Utilities|LinetraceDiminish _outhit)))
    (if (Variables|/Game/Blueprints/BP_Interactable.BP_Interactable_C|GetCanInteract _asbp_interactable)
      (Default|UpdateColor _asbp_interactable)
      (else
        (Development|PrintString "Is Currently Changing Colors")))))

(fn ConstructionScript)